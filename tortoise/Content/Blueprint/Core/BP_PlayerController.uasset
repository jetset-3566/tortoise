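; Player controller that shows the mouse cursor, adds the letter-change widget to the viewport and lets the player click spawn points to spawn animals.
; A left click traces under the cursor on the Visibility channel and calls TrySpawnAnimal on the BP_SpawnPoint hit.
; CheckHoveredUnderCursor uses the same trace to toggle the spawn point hover effect, tracking the highlighted actor.
; BeginPlay also starts a fast looping timer, presumably to poll that hover check.
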(event EventBeginPlay
  (Variables|Default|SetbShowMouseCursor true)
  (Utilities|Time|SetTimerbyEvent (EventDispatchers|CreateEvent :!event CheckHoveredUnderCursor) 0.1 true)
  (bind _returnvalue (UserInterface|CreateWidget "/Game/Blueprint/BPW_LetterChange.BPW_LetterChange_C"))
  (UserInterface|Viewport|AddtoViewport _returnvalue 0))

(event Input|MouseEvents|LeftMouseButton
  (params (Key :type Key%20Structure :default "None"))
  (bind (_hitresult _returnvalue) (Game|Player|GetHitResultUnderCursorbyChannel "TraceTypeQuery1" true))
  (:Pressed
    (if _returnvalue
      (bind _asbp_spawn_point (Utilities|Casting|CastToBP_SpawnPoint (.HitActor (Collision|BreakHitResult _hitresult))))
      (Default|TrySpawnAnimal _asbp_spawn_point))))

(fn ConstructionScript)

(fn CheckHoveredUnderCursor
  (bind (_hitresult _returnvalue) (Game|Player|GetHitResultUnderCursorbyChannel "TraceTypeQuery1" true))
  (bind _hitactor (Collision|BreakHitResult _hitresult))
  (if _returnvalue
    (Utilities|IsValid (Variables|Default|GetHoveredActor)
      (:Is%20Valid
        (if (== (Variables|Default|GetHoveredActor) _hitactor)
          (bind _asbp_spawn_point (Utilities|Casting|CastToBP_SpawnPoint _hitactor :!label _label))
          (Default|SwitchHoveredEffect _asbp_spawn_point true)
          (Variables|Default|SetHoveredActor _asbp_spawn_point)
          (else
            (Utilities|IsValid (Variables|Default|GetHoveredActor) :!label _label_2
              (:Is%20Valid
                (Default|SwitchHoveredEffect (Variables|Default|GetHoveredActor) false)
                (Variables|Default|SetHoveredActor 0))))))
      (:Is%20Not%20Valid
        (goto _label)))
    (else
      (goto _label_2))))