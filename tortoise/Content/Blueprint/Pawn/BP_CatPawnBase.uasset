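; Base cat character that walks to a destination point and dies on arrival.
; BeginPlay applies the configured mesh; StartWalk faces the destination, issues an AI MoveTo and calls MoveLogicPattern, which sets max walk speed.
; On a successful move it stops, plays a death montage with a meow, then destroys itself with an explosion effect when the montage completes.
; Accessors expose movement direction and the destination point.
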(event Custom|StartWalk
  (bind _destinationpoint (Variables|Default|GetDestinationPoint))
  (Transformation|SetActorRotation (Math|Rotator|FindLookatRotation (Transformation|GetActorLocation) _destinationpoint))
  (AI|AIMoveTo self _destinationpoint 0 5.0 false
    (:then
      (CallFunction|MoveLogicPattern))
    (:OnSuccess
      (Components|Movement|StopMovementImmediately (Variables|Character|GetCharacterMovement))
      (Animation|Montage|PlayMontage (Variables|Character|GetMesh) "/Game/LowPoly_Cat/Animations/Anim_Cat_Death_L_Montage.Anim_Cat_Death_L_Montage"
        (:then
          (Audio|SpawnSoundatLocation "/Game/FarmAnimalSounds/Animals/Cat/cue/Cat_Meow_01_Cue.Cat_Meow_01_Cue" (Transformation|GetWorldLocation (Variables|Character|GetMesh)) "0, 0, 0" 1.0 1.0 0.0 0 0))
        (:OnCompleted
          (Actor|DestroyActor)
          (Effects|SpawnEmitteratLocation "/Game/LAT/Effects/P_Proj_Chicken_Imp_Explo_01.P_Proj_Chicken_Imp_Explo_01" (Transformation|GetActorLocation)))))))

(event Custom|MoveLogicPattern
  (Variables|/Script/Engine.CharacterMovementComponent|SetMaxWalkSpeed (Variables|Character|GetCharacterMovement) (Variables|SettingMovePattern|GetMax%20Walk%20Speed)))

(event EventBeginPlay
  (Class|SkinnedMeshComponent|SetSkeletalMesh (Variables|Character|GetMesh) (Variables|Default|GetCurrentMesh) true))

(fn ConstructionScript)

(fn GetMovementDirection
  (return (Variables|Default|GetMovementDirection)))

(fn SetMovementDirection
  (params (MovementDirection :type EMovementDirection%20Enum :default "NewEnumerator0"))
  (Variables|Default|SetMovementDirection MovementDirection)
  (return))

(fn GetDestinationPoint
  (return (Variables|Default|GetDestinationPoint)))