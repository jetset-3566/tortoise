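; Cat pawn variant, apparently a child of a cat pawn base, that moves in a repeating walk-then-pause pattern.
; MoveLogicPattern runs the parent logic, then starts a timer for the first walk phase.
; Two one-shot timers re-arm each other, alternately zeroing CharacterMovement's max walk speed and restoring it from MaxWalkSpeed, with separate durations for each phase.
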(event Custom|WalkMoveEnd
  (Variables|/Script/Engine.CharacterMovementComponent|SetMaxWalkSpeed (Variables|Character|GetCharacterMovement) 0.0)
  (Utilities|Time|SetTimerbyEvent (delegate Custom|PauseMoveEnd) (Variables|Default|GetSecondMovePatternTimer)))

(event Custom|PauseMoveEnd
  (Variables|/Script/Engine.CharacterMovementComponent|SetMaxWalkSpeed (Variables|Character|GetCharacterMovement) (Variables|Default|GetMax%20Walk%20Speed))
  (Utilities|Time|SetTimerbyEvent (delegate Custom|WalkMoveEnd) (Variables|Default|GetFirstMovePatternTimer)))

(event EventBeginPlay
  (|CallParentFunction) ; This node is disabled and will not be called.\nDrag off pins to build functionality.
)

(event Collision|EventActorBeginOverlap
  (params (OtherActor :type Actor%20Object%20Reference))
  (|CallParentFunction OtherActor) ; This node is disabled and will not be called.\nDrag off pins to build functionality.
)

(event EventMoveLogicPattern
  (|CallParentFunction)
  (Utilities|Time|SetTimerbyEvent (delegate Custom|WalkMoveEnd) (Variables|Default|GetFirstMovePatternTimer)))

(fn ConstructionScript
  (|CallParentFunction))