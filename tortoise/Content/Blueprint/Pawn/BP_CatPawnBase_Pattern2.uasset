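; Cat pawn variant that overrides the parent's move logic with a second pattern alternating between advancing and backing up.
; After the parent logic runs, a timer fires a short AI move directly opposite the capsule's forward vector.
; A second timer then switches the movement direction and sends the pawn to its destination point, re-arming the first timer to loop the pattern.
; Both timers start when each move is issued, without waiting for arrival.
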(event Custom|WalkMoveEnd
  (CallFunction|SetMovementDirection "NewEnumerator0")
  (AI|AIMoveTo self (+ (Transformation|GetActorLocation) (* (Math|Vector|GetForwardVector (Variables|Default|GetCapsuleComponent)) -1e+02)) 0 5.0 false
    (:then
      (Utilities|Time|SetTimerbyEvent (delegate Custom|BackMoveEnd) (Variables|Default|GetSecondMovePatternTimer)))))

(event Custom|BackMoveEnd
  (CallFunction|SetMovementDirection "NewEnumerator1")
  (bind _destinationpoint (CallFunction|GetDestinationPoint))
  (AI|AIMoveTo self _destinationpoint 0 5.0 false
    (:then
      (Utilities|Time|SetTimerbyEvent (delegate Custom|WalkMoveEnd) (Variables|Default|GetFirstMovePatternTimer)))))

(event EventBeginPlay
  (|CallParentFunction))

(event Collision|EventActorBeginOverlap
  (params (OtherActor :type Actor%20Object%20Reference))
  (|CallParentFunction OtherActor) ; This node is disabled and will not be called.\nDrag off pins to build functionality.
)

(event EventMoveLogicPattern
  (|CallParentFunction)
  (Utilities|Time|SetTimerbyEvent (delegate Custom|WalkMoveEnd) (Variables|Default|GetFirstMovePatternTimer)))

(fn ConstructionScript
  (|CallParentFunction))