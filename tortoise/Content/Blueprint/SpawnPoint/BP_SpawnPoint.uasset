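; Spawn point that shows a randomly chosen, idle-animated preview animal and spawns it as a pawn on request, with a hover particle effect.
; TrySpawnAnimal is gated by a looping cooldown timer, whose valid handle blocks spawning while a static mesh scales back up as progress.
; The spawned pawn gets the preview mesh and destination, leaps along a spline via a timeline with montage, sound and particles, then starts walking.
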(event Custom|SwitchHoveredEffect
  (params (NewState :type Boolean))
  (bind _particlesystem_hovered (Variables|Default|GetParticleSystem_Hovered))
  (bind _returnvalue (Components|Activation|IsActive _particlesystem_hovered))
  (Rendering|SetVisibility _particlesystem_hovered NewState false)
  (if NewState
    (if (not _returnvalue)
      (Components|Activation|Activate _particlesystem_hovered true))
    (elif _returnvalue
      (Components|Activation|Deactivate _particlesystem_hovered))))

(event Custom|TrySpawnAnimal
  (bind _bisbusy (CallFunction|CheckCoolDown))
  (if _bisbusy
    (Development|PrintString "WaitCoolDown")
    (else
      (Variables|CoolDown|SetCurrentCoolDown 1.0)
      (bind _returnvalue (Utilities|Time|SetTimerbyFunctionName 0 "CoolDownTimer" 0.1 true))
      (Variables|CoolDown|SetCoolDownTimer_Handle _returnvalue)
      (Transformation|SetRelativeScale3D (Variables|Default|GetStaticMesh) "0.010000,0.010000,0.010000")
      (CallFunction|SpawnAnimal)
      (CallFunction|ResetSettingSpawnPoint))))

(event Custom|SpawnAnimal
  (bind _spawnpoint (Variables|Default|GetSpawnPoint))
  (bind _spawnpoint_2 (Variables|Default|GetSpawnPoint))
  (bind _returnvalue (Transformation|GetWorldLocation _spawnpoint_2))
  (bind _returnvalue_2 (Game|SpawnActorfromClass (Variables|Settings|GetPawnToSpawn) (Math|Transform|MakeTransform (Transformation|GetWorldLocation _spawnpoint) (Transformation|GetWorldRotation _spawnpoint) "1,1,1") "AlwaysSpawn" (Game|GetPlayerController 0) (Variables|Settings|GetCurrentSelectedMeshes) (Transformation|GetWorldLocation (Variables|Default|GetDestinationPoint)) 0))
  (Audio|SpawnSoundatLocation "/Game/FarmAnimalSounds/Animals/Cat/cue/Cat_Meow_01_Cue.Cat_Meow_01_Cue" _returnvalue "0, 0, 0" 1.0 1.0 0.0 0 0)
  (Effects|SpawnEmitteratLocation "/Game/LAT/Effects/P_Proj_Chicken_Imp_Explo_01.P_Proj_Chicken_Imp_Explo_01" _returnvalue)
  (Animation|Montage|PlayMontage (Variables|/Script/Engine.Character|GetMesh _returnvalue_2) "/Game/LowPoly_Cat/Animations/Anim_Cat_Jump_trot_IP_Montage.Anim_Cat_Jump_trot_IP_Montage"
    (:then
      (bind _newtrack_0 (Timeline|JumpSpline Play)
        (:Update
          (Transformation|SetActorLocation _returnvalue_2 (Spline|GetLocationatTime (Variables|Default|GetSpline) _newtrack_0 "World" false) false false))
        (:Finished
          (Default|StartWalk _returnvalue_2))))))

(event Custom|ResetSettingSpawnPoint
  (Variables|Settings|SetCurrentSelectedMeshes (.OutItem (Utilities|Array|Random (Variables|Settings|GetSkeletalMeshes))))
  (Class|SkinnedMeshComponent|SetSkeletalMesh (Variables|Default|GetSkeletalMesh) (Variables|Settings|GetCurrentSelectedMeshes) true)
  (Transformation|SetRelativeRotation (Variables|Default|GetSkeletalMesh) (Math|Rotator|MakeRotator 0.0 0.0 (Math|Random|RandomFloatinRange -3e+01 -1.6e+02)) false false)
  (Components|Animation|PlayAnimation (Variables|Default|GetSkeletalMesh) (.OutItem (Utilities|Array|Random (Variables|Settings|GetAnimSequensesIdle))) true))

(event EventBeginPlay
  (Components|Activation|Deactivate (Variables|Default|GetParticleSystem_Hovered))
  (CallFunction|ResetSettingSpawnPoint))

(fn ConstructionScript)

(fn CheckCoolDown
  (return (Utilities|Time|IsValidTimerHandle (Variables|CoolDown|GetCoolDownTimer_Handle))))

(fn CoolDownTimer
  (bind _staticmesh (Variables|Default|GetStaticMesh))
  (bind _output_get (Variables|CoolDown|SetCurrentCoolDown (- (Variables|CoolDown|GetCurrentCoolDown) (Variables|CoolDown|GetStepCoolDown))))
  (if (<= _output_get 0.0)
    (Utilities|Time|ClearandInvalidateTimerbyHandle (Variables|CoolDown|GetCoolDownTimer_Handle))
    (Transformation|SetRelativeScale3D _staticmesh "1.000000,1.000000,1.000000")
    (else
      (Transformation|SetRelativeScale3D _staticmesh (Math|Conversions|ToVector(Float) (Math|Float|Absolute(Float) (- _output_get 1.0)))))))